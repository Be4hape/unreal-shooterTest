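; BGM is a Blueprint that switches background music between exploration and combat.
; It starts with BGM1 as the sound on its AudioComponent at BeginPlay.
; Every Tick it polls the current-state enum (게임현재상태) on MyGameStateBase, selecting BGM1 for 탐험 (exploration) and BGM2 for 전투 (combat).
; It calls SetSound only when the assigned track differs, with no fade or crossfade.
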(event EventBeginPlay
  (Audio|Components|Audio|SetSound (Variables|Components|GetAudioComponent) "/Game/BGM/BGM1.BGM1"))

(event EventTick
  (params (DeltaSeconds :type Float%20%28single-precision%29))
  (bind _asmy_game_state_base (Utilities|Casting|CastToMyGameStateBase (Game|GetGameState)))
  (switch Utilities|FlowControl|Switch|Switchon게임상태 (Variables|/Game/Blueprints/MyGameStateBase.MyGameStateBase_C|Get게임현재상태 _asmy_game_state_base)
    (:NewEnumerator0
      (if (!= (Variables|/Script/Engine.AudioComponent|GetSound (Variables|Components|GetAudioComponent)) "/Game/BGM/BGM1.BGM1")
        (Audio|Components|Audio|SetSound (Variables|Components|GetAudioComponent) "/Game/BGM/BGM1.BGM1")))
    (:NewEnumerator1
      (if (!= (Variables|/Script/Engine.AudioComponent|GetSound (Variables|Components|GetAudioComponent)) "/Game/BGM/BGM2.BGM2")
        (Audio|Components|Audio|SetSound (Variables|Components|GetAudioComponent) "/Game/BGM/BGM2.BGM2")))))

(fn ConstructionScript)