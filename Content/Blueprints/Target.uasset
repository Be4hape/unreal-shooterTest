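; Target actor that reacts to incoming damage by reporting the extra elemental damage of a missile hit.
; AnyDamage casts the damage type to MyDamageType, calls its elemental damage function with fixed fire and poison resistances, and prints the result without applying it to health.
; Disconnected leftover logic would decrement Hp and destroy the actor at zero, or set the game state on MyGameStateBase, but never runs.
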(event EventBeginPlay)

(event Collision|EventActorBeginOverlap
  (params (OtherActor :type Actor%20Object%20Reference)))

(event EventTick
  (params (DeltaSeconds :type Float%20%28single-precision%29)))

(event Game|Damage|EventAnyDamage
  (params (Damage :type Float%20%28single-precision%29) (DamageType :type Damage%20Type%20Object%20Reference) (InstigatedBy :type Controller%20Object%20Reference) (DamageCauser :type Actor%20Object%20Reference))
  (bind _asmy_damage_type (Utilities|Casting|CastToMyDamageType DamageType))
  (bind __전체속성피해 (Default|속성피해적용 _asmy_damage_type 5.0 5.0))
  (Development|PrintText (Utilities|Text|FormatText "미사일 속성 추가 피해 {d}" __전체속성피해)))

(fn ConstructionScript)