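; Motionguns is a rotating gun Blueprint that continuously fires Missile actors from two fire points.
; Each Tick, RotateBase yaws the Base component by RotSpeed scaled by delta time for frame-rate-independent spin.
; FireMissile then spawns a Missile at the world transform of FirePoint1 and FirePoint2.
; Firing has no timer or cooldown, so the spawn rate follows the frame rate.
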(event EventBeginPlay)

(event Collision|EventActorBeginOverlap
  (params (OtherActor :type Actor%20Object%20Reference)))

(event EventTick
  (params (DeltaSeconds :type Float%20%28single-precision%29))
  (CallFunction|RotateBase DeltaSeconds) ; 베이트 컴포넌트 회전함수
  ;[0.2051 0.1521 1 1 12] 미사일 액터 발사하기
  (CallFunction|FireMissile (Variables|Default|GetFirePoint1))
  (CallFunction|FireMissile (Variables|Default|GetFirePoint2)))

(event EventEndPlay
  (params (EndPlayReason :type EEndPlayReason%20Enum :default "Destroyed")))

(fn ConstructionScript)

(fn RotateBase
  (params (Delta%20Seconds :type Float%20%28single-precision%29))
  (Transformation|AddLocalRotation (Variables|Default|GetBase) (Math|Rotator|MakeRotator 0.0 0.0 (* Delta%20Seconds (Variables|Default|GetRotSpeed))) false false)
  (return 0.0 0.0 0.0))

(fn FireMissile
  (params (FirePoint :type Child%20Actor%20Component%20Object%20Reference))
  (Game|SpawnActorfromClass "/Game/Blueprints/Missile.Missile_C" (Transformation|GetWorldTransform FirePoint) "Undefined" 0 0))