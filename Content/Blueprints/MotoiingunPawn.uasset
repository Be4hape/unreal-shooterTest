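; MotoiingunPawn is a player-controlled gun pawn that rotates its base and fires missiles from four fire points.
; Tick yaws Base from the 회전 axis, then sets its rotation through ClampBaseRotator, whose yaw-clamp node appears unconnected.
; The 발사 action loops over the fire points, spawning a Missile, playing audio and setting the MyGameStateBase game state at each.
; Left/right axis events only store values; their limited-rotation logic is disconnected.
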(event EventBeginPlay
  (Variables|Default|SetFirePositions (Utilities|Array|MakeArray (Variables|Default|GetFirePosition0) (Variables|Default|GetFirePosition1) (Variables|Default|GetFirePosition2) (Variables|Default|GetFirePosition3)))
  (Development|PrintString "발사위치 배열 만들기"))

(event Collision|EventActorBeginOverlap
  (params (OtherActor :type Actor%20Object%20Reference)))

(event EventTick
  (params (DeltaSeconds :type Float%20%28single-precision%29))
  (Transformation|AddLocalRotation (Variables|Default|GetBase) (Math|Rotator|MakeRotator 0.0 0.0 (* DeltaSeconds (Input|AxisValues|Get회전) (Variables|Default|GetSpeed))) false false) ; 노드별 주석 : 로칼회전
  (Transformation|SetWorldRotation (Variables|Default|GetBase) (Utilities|ClampBaseRotator) false false))

(event Input|ActionEvents|InputAction발사
  (params (Key :type Key%20Structure :default "None"))
  (:Pressed
    (for _array_element (Variables|Default|GetFirePositions)
      (Game|SpawnActorfromClass "/Game/Blueprints/Missile.Missile_C" (Transformation|GetWorldTransform _array_element) "Undefined" 0 0)
      (Audio|Components|Audio|Play (Variables|Default|GetAudio) 0.0)
      (bind _asmy_game_state_base (Utilities|Casting|CastToMyGameStateBase (Game|GetGameState)))
      (Variables|/Game/Blueprints/MyGameStateBase.MyGameStateBase_C|Set게임현재상태 _asmy_game_state_base "NewEnumerator1"))))

(event Input|AxisEvents|InputAxis회전
  (params (AxisValue :type Float%20%28single-precision%29)))

(event Input|AxisEvents|InputAxis오른쪽회전
  (params (AxisValue :type Float%20%28single-precision%29))
  ;[0.2886 0.236 1] Base 오른쪽 회전
  (Variables|Default|SetRight%20Axis%20Value AxisValue))

(event Input|AxisEvents|InputAxis왼쪽회전
  (params (AxisValue :type Float%20%28single-precision%29))
  ;[1 0.0831 0.103] Base 회쪽회전
  (Variables|Default|SetLeft%20Axis%20Value AxisValue))

(fn ConstructionScript)